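; Player-flyable Eurofighter jet with engine toggle, ground taxi, takeoff, flight and landing, flagging when the ThirdPersonCharacter is within boarding range.
; Axis inputs steer and set thrust, feeding smoothed movement plus wheel and control-surface rotations.
; Tick scales exhausts, manages camera lag and rechargeable nitro, and updates the HUD.
; A downward trace lands the jet when gear is down, roll is level and thrust is minimal.
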(event `self.ReceiveBeginPlay`
  (`|ExecutionSequence`
    (:`then_0`
      (set `self.Target Thrust Speed` (`self.Minimum Thrust Speed`))
      ;[1 1 1] 착륙 Z
      (set `self.Start Z Offset` 131.0)
      ;[1 1 1] UI 생성
      (bind _returnvalue (`|CreateWidget` "/Game/_My/EuroFighter/UI/EuroFighter_UI.EuroFighter_UI_C"))
      (bind _output_get (set `self.HUD_Ref` _returnvalue))
      (`UserWidget.AddToViewport` _output_get 0))
    (:`then_1`
      ;[1 1 1] 파티클
      (`SceneComponent.SetRelativeScale3D` (`self.LeftExhaust`) (0.0 0.0 0.0))
      (`SceneComponent.SetRelativeScale3D` (`self.RightExhaust`) (0.0 0.0 0.0)))))

(event `self.ReceiveTick`
  (params (DeltaSeconds :type "Float (single-precision)"))
  (bind (_returnvalue_x _returnvalue_y) (`KismetMathLibrary.BreakVector` (`self.K2_GetActorLocation`)))
  (bind _returnvalue_roll (`KismetMathLibrary.BreakRotator` (`self.K2_GetActorRotation`)))
  (bind _returnvalue_roll_2 (`KismetMathLibrary.BreakRotator` (`self.K2_GetActorRotation`)))
  (bind _hud_ref (`self.HUD_Ref`))
  (bind _leftexhaust (`self.LeftExhaust`))
  (bind _nitro_ (`self.Nitro?`))
  (bind _returnvalue (`KismetMathLibrary.NormalizeToRange` (`self.Current Thrust Speed`) 0.0 (`self.Maximum Thrust Speed`)))
  (bind _speedtext (`/Game/_My/EuroFighter/UI/EuroFighter_UI.SpeedText` (`self.HUD_Ref`)))
  (bind _crosshair (`/Game/_My/EuroFighter/UI/EuroFighter_UI.Crosshair` (`self.HUD_Ref`)))
  (bind _speedmeter (`/Game/_My/EuroFighter/UI/EuroFighter_UI.SpeedMeter` _hud_ref))
  (bind _meterpoint (`/Game/_My/EuroFighter/UI/EuroFighter_UI.MeterPoint` _hud_ref))
  (bind _landingsign (`/Game/_My/EuroFighter/UI/EuroFighter_UI.landingsign` (`self.HUD_Ref`)))
  (bind _flysign (`/Game/_My/EuroFighter/UI/EuroFighter_UI.flysign` (`self.HUD_Ref`)))
  (bind _speedprogressbar (`/Game/_My/EuroFighter/UI/EuroFighter_UI.SpeedProgressBar` (`self.HUD_Ref`)))
  (bind _returnvalue_2 (- (`KismetMathLibrary.Round` (`self.Target Thrust Speed`)) 5000))
  (bind (_font_fontobject _font_fontmaterial _font_outlinesettings _font_typefacefontname _font_size _font_letterspacing) (break `SlateFontInfo` (`TextBlock.Font` _speedtext)))
  (`|ExecutionSequence`
    (:`then_0`
      ;[1 1 1] Ground Move
      (if (`self.EngineStart?`)
        (bind _output_get (set `self.Move Forward Interp` (`KismetMathLibrary.FClamp` (`KismetMathLibrary.FInterpTo` (stale _output_get) (`self.GetInputAxisValue`) (`GameplayStatics.GetWorldDeltaSeconds`) 0.25))))
        (if (> (`self.Move Forward Interp`) 0.0)
          (`ActorComponent.Activate` _leftexhaust false)
          (`ActorComponent.Activate` (`self.RightExhaust`) false)
          (else
            (`ActorComponent.Deactivate` _leftexhaust)
            (`ActorComponent.Deactivate` (`self.RightExhaust`))))
        ;[1 1 1] 스피드 비례 이펙트
        (`SceneComponent.SetRelativeScale3D` (`self.LeftExhaust`) (`KismetMathLibrary.VInterpTo` (`SceneComponent.RelativeScale3D` (`self.RightExhaust`)) (`KismetMathLibrary.SelectVector` (`KismetMathLibrary.MakeVector` _returnvalue _returnvalue _returnvalue) (0.0 0.0 0.0) (`self.Flying?`)) (`GameplayStatics.GetWorldDeltaSeconds`) (`KismetMathLibrary.SelectFloat` 4.0 0.5 (`self.Flying?`))))
        (`SceneComponent.SetRelativeScale3D` (`self.RightExhaust`) (`KismetMathLibrary.VInterpTo` (`SceneComponent.RelativeScale3D` (`self.RightExhaust`)) (`KismetMathLibrary.SelectVector` (`KismetMathLibrary.MakeVector` _returnvalue _returnvalue _returnvalue) (0.0 0.0 0.0) (`self.Flying?`)) (`GameplayStatics.GetWorldDeltaSeconds`) (`KismetMathLibrary.SelectFloat` 4.0 0.5 (`self.Flying?`))))))
    (:`then_1`
      ;[1 1 1] 비행
      (if (`self.Flying?`)
        (`self.Add Flight Movement`)
        (`KismetSystemLibrary.Delay` 0.2)
        (`self.Landing Trace` "ForOneFrame" (`self.Start Z Offset`))))
    (:`then_2`
      (`self.Set Camera Lag`))
    (:`then_3`
      (`|ExecutionSequence`
        (:`then_0`
          (`TextBlock.SetText` _speedtext (`KismetTextLibrary.Conv_StringToText` (`KismetStringLibrary.Concat_StrStr` (`KismetTextLibrary.Conv_TextToString` (`KismetTextLibrary.Conv_IntToText` _returnvalue_2)) " 스로틀")))
          (if (`self.EngineStart?`)
            (`TextBlock.SetOpacity` _speedtext 1.0)
            (else
              (`TextBlock.SetOpacity` _speedtext 0.0)))
          (`TextBlock.SetFont` _speedtext (make `SlateFontInfo` _font_fontobject _font_fontmaterial _font_outlinesettings _font_typefacefontname (`KismetMathLibrary.SelectInt` 19 18 (< _returnvalue_2 10000)) _font_letterspacing))
          (`ProgressBar.SetPercent` _speedprogressbar (`KismetMathLibrary.FInterpTo` (`ProgressBar.Percent` _speedprogressbar) (`KismetMathLibrary.NormalizeToRange` (`self.Target Thrust Speed`) (`self.Minimum Thrust Speed`) (`self.Maximum Thrust Speed`)) (`GameplayStatics.GetWorldDeltaSeconds`) 4.5))
          (if (`self.EngineStart?`)
            (`Widget.SetRenderOpacity` _speedprogressbar 1.0)
            (else
              (`Widget.SetRenderOpacity` _speedprogressbar 0.0))))
        (:`then_1`
          (`Widget.SetRenderTranslation` _crosshair (`KismetMathLibrary.MakeVector2D` (`KismetMathLibrary.FClamp` (`KismetMathLibrary.FInterpTo` (`KismetMathLibrary.BreakVector2D` (break `WidgetTransform` (`Widget.RenderTransform` (`/Game/_My/EuroFighter/UI/EuroFighter_UI.Crosshair` (`self.HUD_Ref`))))) (`KismetMathLibrary.SelectFloat` (* (`self.GetInputAxisValue`) 150.0) 0.0 (`self.Flying?`)) (`GameplayStatics.GetWorldDeltaSeconds`) 2.0) -150.0 150.0) (`KismetMathLibrary.FClamp` (`KismetMathLibrary.FInterpTo` (`.Y` (`KismetMathLibrary.BreakVector2D` (break `WidgetTransform` (`Widget.RenderTransform` (`/Game/_My/EuroFighter/UI/EuroFighter_UI.Crosshair` (`self.HUD_Ref`)))))) (`KismetMathLibrary.SelectFloat` (* (`self.GetInputAxisValue`) (`KismetMathLibrary.SelectFloat` 150.0 -150.0 (`self.Invert Vertical Flight`))) 0.0 (`self.Flying?`)) (`GameplayStatics.GetWorldDeltaSeconds`) 2.0) -150.0 150.0)))
          (`Widget.SetRenderTranslation` (`/Game/_My/EuroFighter/UI/EuroFighter_UI.Rotate` (`self.HUD_Ref`)) (`KismetMathLibrary.MakeVector2D` (`KismetMathLibrary.FClamp` (`KismetMathLibrary.FInterpTo` (`KismetMathLibrary.BreakVector2D` (break `WidgetTransform` (`Widget.RenderTransform` (`/Game/_My/EuroFighter/UI/EuroFighter_UI.Crosshair` (`self.HUD_Ref`))))) (`KismetMathLibrary.SelectFloat` (* (`self.GetInputAxisValue`) 150.0) 0.0 (`self.Flying?`)) (`GameplayStatics.GetWorldDeltaSeconds`) 2.0) -150.0 150.0) (`KismetMathLibrary.FClamp` (`KismetMathLibrary.FInterpTo` (`.Y` (`KismetMathLibrary.BreakVector2D` (break `WidgetTransform` (`Widget.RenderTransform` (`/Game/_My/EuroFighter/UI/EuroFighter_UI.Crosshair` (`self.HUD_Ref`)))))) (`KismetMathLibrary.SelectFloat` (* (`self.GetInputAxisValue`) (`KismetMathLibrary.SelectFloat` 150.0 -150.0 (`self.Invert Vertical Flight`))) 0.0 (`self.Flying?`)) (`GameplayStatics.GetWorldDeltaSeconds`) 2.0) -150.0 150.0)))
          (if (`self.EngineStart?`)
            (`Image.SetOpacity` _crosshair 1.0)
            (`Image.SetOpacity` (`/Game/_My/EuroFighter/UI/EuroFighter_UI.Rotate` (`self.HUD_Ref`)) 1.0)
            (else
              (`Image.SetOpacity` _crosshair 0.0)
              (`Image.SetOpacity` (`/Game/_My/EuroFighter/UI/EuroFighter_UI.Rotate` (`self.HUD_Ref`)) 0.0)))
          (`Widget.SetRenderTransformAngle` (`/Game/_My/EuroFighter/UI/EuroFighter_UI.Rotate` (`self.HUD_Ref`)) _returnvalue_roll_2))
        (:`then_2`
          (`Widget.SetRenderTransformAngle` (`/Game/_My/EuroFighter/UI/EuroFighter_UI.MeterPoint` (`self.HUD_Ref`)) (`KismetMathLibrary.FInterpTo` 0.0 (`KismetMathLibrary.SelectFloat` (`KismetMathLibrary.SelectFloat` 120.0 (`KismetMathLibrary.MapRangeClamped` (`self.Current Thrust Speed`) 0.0 (`self.Maximum Thrust Speed`) -120.0 60.0) (`self.Nitro?`)) (`KismetMathLibrary.MapRangeClamped` (`self.Move Forward Interp`) 0.0 1.0 -120.0 -90.0) (`self.Flying?`)) (`GameplayStatics.GetWorldDeltaSeconds`)))
          (if (`self.EngineStart?`)
            (`Image.SetOpacity` _speedmeter 1.0)
            (`Image.SetOpacity` _meterpoint 1.0)
            (else
              (`Image.SetOpacity` _speedmeter 0.0)
              (`Image.SetOpacity` _meterpoint 0.0))))
        (:`then_3`
          (`self.Set Altitude Level`))
        (:`then_4`
          (if (`self.Flying?`)
            (if (== (`self.Minimum Thrust Speed`) (`KismetMathLibrary.FInterpTo` 0.0 (`self.Target Thrust Speed`) (`GameplayStatics.GetWorldDeltaSeconds`)))
              (if (`self.InsertWheel`)
                (`Image.SetOpacity` _landingsign 0.0 :!label _label)
                (elif (`KismetMathLibrary.InRange_FloatFloat` _returnvalue_roll -8.0 8.0)
                  (`Image.SetOpacity` _landingsign 1.0)
                  (else
                    (goto _label))))
              (else
                (goto _label)))
            (else
              (goto _label))))
        (:`then_5`
          (if (`self.Ready To Fly`)
            (if (`self.Flying?`)
              (`Image.SetOpacity` _flysign 0.0 :!label _label_2)
              (else
                (`Image.SetOpacity` _flysign 1.0)))
            (else
              (goto _label_2))))))
    (:`then_4`
      ;[1 1 1] 탑승거리
      (bind _asthird_person_character (cast `/Game/_My/Player/ThirdPersonCharacter` (`GameplayStatics.GetPlayerCharacter` 0)))
      (bind (_returnvalue_x_2 _returnvalue_y_2) (`KismetMathLibrary.BreakVector` (`self.K2_GetActorLocation` _asthird_person_character)))
      (if (and (`KismetMathLibrary.InRange_FloatFloat` (- _returnvalue_x_2 _returnvalue_x) -600.0 600.0) (`KismetMathLibrary.InRange_FloatFloat` (- _returnvalue_y_2 _returnvalue_y) -600.0 600.0))
        (set `/Game/_My/Player/ThirdPersonCharacter.InRange_EuroFighter` true _asthird_person_character)
        (else
          (set `/Game/_My/Player/ThirdPersonCharacter.InRange_EuroFighter` false _asthird_person_character))))
    (:`then_5`
      ;[1 1 1] Nitro Speed 리셋
      (`|ExecutionSequence`
        (:`then_0`
          (bind _output_get_2 (set `self.Nitro Level` (`KismetMathLibrary.FInterpTo_Constant` (stale _output_get_2) (`KismetMathLibrary.SelectFloat` 0.0 1.0 _nitro_) (`GameplayStatics.GetWorldDeltaSeconds`) (`KismetMathLibrary.SelectFloat` 0.1 0.05 _nitro_))))
          (`ProgressBar.SetPercent` (`/Game/_My/EuroFighter/UI/EuroFighter_UI.NitroBar` (`self.HUD_Ref`)) _output_get_2)
          (if (== _output_get_2 0.0)
            (bind _output_get_3 (set `self.Maximum Thrust Speed` 25000.0))
            (set `self.Target Thrust Speed` _output_get_3)
            (set `self.Nitro?` false)))))))

(event `Key|C`
  (params (Key :type "Key Structure"))
  ;[1 0.1428 0] 바퀴 제어
  (:`Pressed`
    (if (`self.Flying?`)
      (if (`self.InsertWheel`)
        (set `self.InsertWheel` false)
        (else
          (set `self.InsertWheel` true))))))

(event `Key|J`
  (params (Key :type "Key Structure"))
  ;[1 0.1789 0.02901] 시동걸기
  (:`Pressed`
    (if (`self.Flying?`)
      _
      (elif (== (`self.Move Forward Interp`) 0.0)
        (if (`self.EngineStart?`)
          (set `self.EngineStart?` false)
          (else
            (set `self.EngineStart?` true)))))))

(event `InputAxis|MoveForward`
  (params (AxisValue :type "Float (single-precision)"))
  (bind _wheel_rotation_side_max (`self.Wheel Rotation side Max`))
  (bind (_wheel_rotation_roll _wheel_rotation_pitch _wheel_rotation_yaw) (`KismetMathLibrary.BreakRotator` (`self.Wheel Rotation`)))
  (bind _returnvalue (> (`self.Move Forward Interp`) 0.9))
  (bind (_returnvalue_roll _returnvalue_pitch) (`KismetMathLibrary.BreakRotator` (`SceneComponent.GetSocketRotation` (`self.SK_West_Fighter_Typhoon`) "front_wheel_jnt")))
  ;[0.1797 0.3214 1] MoveForward
  ;;[1 1 1] 비행 여부
  (if (`self.EngineStart?`)
    (if (`self.Flying?`)
      (if (not (`self.Nitro?`))
        (set `self.Target Thrust Speed` (`KismetMathLibrary.FClamp` (+ (* AxisValue (`GameplayStatics.GetWorldDeltaSeconds`) 2000.0) (`self.Target Thrust Speed`)) (`self.Minimum Thrust Speed`) (`self.Maximum Thrust Speed`)))
        (if (not (`self.Flying?`)) :!label _label_3
          (`|ExecutionSequence`
            (:`then_0`
              ;;[1 1 1] 이륙준비
              (`self.K2_AddActorWorldOffset` (`KismetMathLibrary.MakeVector` (.x (* (`self.GetActorForwardVector`) (* (`self.Move Forward Interp`) (/ (`self.Target Thrust Speed`) 200.0)))) (.y (* (`self.GetActorForwardVector`) (* (`self.Move Forward Interp`) (/ (`self.Target Thrust Speed`) 200.0))))) true)
              (if _returnvalue
                ;;[1 1 1] 속도가 충분할 때 이륙
                (set `self.Ready To Fly` true)
                (else
                  (set `self.Ready To Fly` false)))
              (if (and _returnvalue (`PlayerController.IsInputKeyDown` (`GameplayStatics.GetPlayerController` 0) "SpaceBar"))
                (set `self.Flying?` true)
                (set `SpringArmComponent.bUsePawnControlRotation` false (`self.SpringArm`))
                (`self.K2_AddActorWorldOffset` (0.0 0.0 0.0) true)))
            (:`then_1`
              ;[1 1 1] Wheel Rotation
              (set `self.Wheel Rotation` (`KismetMathLibrary.MakeRotator` 0.0 (+ _returnvalue_pitch (* (`self.Move Forward Interp`) -500.0)) (`KismetMathLibrary.FInterpTo` _wheel_rotation_yaw (`KismetMathLibrary.MapRangeClamped` (`self.GetInputAxisValue`) -1.0 1.0 (* _wheel_rotation_side_max -1.0) _wheel_rotation_side_max) (`GameplayStatics.GetWorldDeltaSeconds`) 0.4)))))))
      (else
        (goto _label_3)))))

(event `InputAxis|LookUp`
  (params (AxisValue :type "Float (single-precision)"))
  (bind _returnvalue (`GameplayStatics.GetWorldDeltaSeconds`))
  (bind _aileron_interrior_rotation_max (`self.Aileron Interrior Rotation Max`))
  (bind _returnvalue_2 (* AxisValue (`KismetMathLibrary.SelectFloat` -1.0 1.0 (`self.Invert Vertical Flight`))))
  ;[0.8162 0.4725 1] LookUp
  (if (`self.Flying?`)
    (bind _output_get (set `self.Flight Pitch` (`KismetMathLibrary.FInterpTo` (stale _output_get) _returnvalue_2 _returnvalue 10.0)))
    (`self.K2_AddActorLocalRotation` (`KismetMathLibrary.MakeRotator` 0.0 (* _output_get _returnvalue (`self.Flight Turn Rate`))))
    (set `self.Aileron Interrior Rotation` (`KismetMathLibrary.MakeRotator` 0.0 (`KismetMathLibrary.MapRangeClamped` (`self.Flight Pitch`) -1.0 1.0 _aileron_interrior_rotation_max (* _aileron_interrior_rotation_max -1.0))))
    (else
      (`self.AddControllerPitchInput` _returnvalue_2))))

(event `InputAxis|Turn`
  (params (AxisValue :type "Float (single-precision)"))
  (bind _returnvalue (`GameplayStatics.GetWorldDeltaSeconds`))
  (bind _back_rudder_rotation_max (`self.Back Rudder Rotation max`))
  ;[0.8162 0.4725 1] Turn
  (if (`self.Flying?`)
    (bind _output_get (set `self.Flight Turn` (`KismetMathLibrary.FInterpTo` (stale _output_get) AxisValue _returnvalue 10.0)))
    (`self.K2_AddActorLocalRotation` (`KismetMathLibrary.MakeRotator` 0.0 0.0 (* _output_get _returnvalue (`self.Flight Turn Rate`))))
    (set `self.Back Rudder Rotation` (`KismetMathLibrary.MakeRotator` 0.0 0.0 (`KismetMathLibrary.MapRangeClamped` (`self.Flight Turn`) -1.0 1.0 _back_rudder_rotation_max (* _back_rudder_rotation_max -1.0))))
    (else
      (`self.AddControllerYawInput` AxisValue))))

(event `InputAxis|MoveRight`
  (params (AxisValue :type "Float (single-precision)"))
  (bind _aileron_interrior_rotation_max (`self.Aileron Interrior Rotation Max`))
  (bind _aileron_interrior_rotation_max_2 (`self.Aileron Interrior Rotation Max`))
  ;[0.1797 0.3214 1] Move Left/Right
  (if (`self.EngineStart?`)
    (if (`self.Flying?`)
      (bind _output_get (set `self.Flight Roll` (`KismetMathLibrary.FInterpTo` (stale _output_get) AxisValue (`GameplayStatics.GetWorldDeltaSeconds`) 10.0)))
      (`self.K2_AddActorLocalRotation` (`KismetMathLibrary.MakeRotator` (* _output_get (`GameplayStatics.GetWorldDeltaSeconds`) 90.0)))
      (set `self.Aileron Flap Rotation Left` (`KismetMathLibrary.MakeRotator` 0.0 (`KismetMathLibrary.MapRangeClamped` (`self.GetInputAxisValue`) -1.0 1.0 _aileron_interrior_rotation_max_2 (* _aileron_interrior_rotation_max_2 -1.0))))
      (set `self.Aileron Flap Rotation Right` (`KismetMathLibrary.MakeRotator` 0.0 (`KismetMathLibrary.MapRangeClamped` (`self.GetInputAxisValue`) -1.0 1.0 (* _aileron_interrior_rotation_max -1.0) _aileron_interrior_rotation_max)))
      (else
        ;;[1 1 1] 지상 좌/우 움직임
        (if (> (`self.GetInputAxisValue`) 0.0)
          (`self.K2_AddActorWorldRotation` (`KismetMathLibrary.MakeRotator` 0.0 0.0 (* AxisValue (`GameplayStatics.GetWorldDeltaSeconds`) 20.0))))))))

(event `Key|LeftShift`
  (params (Key :type "Key Structure"))
  ;[1 0.1719 0.1719] Nitro
  (:`Pressed`
    (if (and (== (`self.Nitro Level`) 1.0) (`self.Flying?`))
      (set `self.Nitro?` true)
      (bind _output_get (set `self.Maximum Thrust Speed` (`self.Nitro Thrust Speed`)))
      (bind _output_get_2 (set `self.Target Thrust Speed` _output_get))
      (set `self.Current Thrust Speed` _output_get_2)
      (`GameplayStatics.SpawnEmitterAttached` "/Game/_My/EuroFighter/VFX/RingBurst.RingBurst" (`self.SK_West_Fighter_Typhoon`) "None" (0.0 0.0 0.0) (struct) (7.0 7.0 7.0)))))

(fn `Add Flight Movement`
  (bind _returnvalue (`GameplayStatics.GetWorldDeltaSeconds`))
  ;[1 1 1] Set Flight Speed
  (bind _output_get (set `self.Current Thrust Speed` (`KismetMathLibrary.FInterpTo` (stale _output_get) (`self.Target Thrust Speed`) _returnvalue 4.0)))
  ;[1 1 1] 비행 전방 움직임
  (`self.K2_AddActorWorldOffset` (* (`SceneComponent.GetForwardVector` (`self.SK_West_Fighter_Typhoon`)) (* _output_get _returnvalue)) true))

(fn `Landing Trace`
  (params (Debug :type "EDrawDebugTrace Enum" :default "None") (`Spawned Z Offset` :type "Float (double-precision)"))
  (bind _returnvalue (`self.K2_GetActorLocation`))
  (bind _returnvalue_roll (`KismetMathLibrary.BreakRotator` (`self.K2_GetActorRotation`)))
  (bind (_returnvalue_roll_2 _returnvalue_pitch _returnvalue_yaw) (`KismetMathLibrary.BreakRotator` (`self.K2_GetActorRotation`)))
  (bind (_outhit _returnvalue_2) (`KismetSystemLibrary.LineTraceSingle` _returnvalue (- _returnvalue (`KismetMathLibrary.MakeVector` 0.0 0.0 `Spawned Z Offset`)) "TraceTypeQuery1" false (`|MakeArray` self :!type "Actor Object Reference") Debug))
  ;[1 1 1] 착륙 가능 여부 -> 속도
  (if _returnvalue_2
    ;[1 1 1] 착륙가능여부 -> 바퀴
    (if (not (`self.InsertWheel`))
      ;[1 1 1] 착륙가능여부 -> 수평
      (if (`KismetMathLibrary.InRange_FloatFloat` _returnvalue_roll -8.0 8.0)
        (if (== (`KismetMathLibrary.MapRangeClamped` (`self.Target Thrust Speed`) (`self.Minimum Thrust Speed`) (`self.Maximum Thrust Speed`) 0.0 1.0) 0.0)
          ;[1 1 1] 착륙
          (set `self.Flying?` false)
          (`self.K2_SetActorRelativeTransform` (`KismetMathLibrary.MakeTransform` (`KismetMathLibrary.VInterpTo` (`self.K2_GetActorLocation`) (+ (`.TraceEnd` (`GameplayStatics.BreakHitResult` _outhit)) (`KismetMathLibrary.MakeVector` 0.0 0.0 (`local.Spawned Z Offset`))) (`GameplayStatics.GetWorldDeltaSeconds`) 3.0) (`KismetMathLibrary.MakeRotator` 0.0 0.0 _returnvalue_yaw)))
          ;[1 1 1] 착륙 변수 설정
          (set `SpringArmComponent.bUsePawnControlRotation` true (`self.SpringArm`))
          (set `self.Move Forward Interp` 1.0))))))

(fn `Set Camera Lag`
  (bind _springarm (`self.SpringArm`))
  (bind _returnvalue (`KismetMathLibrary.SelectFloat` 10.0 500.0 (`self.Flying?`)))
  ;[1 1 1] 착륙 카메라 제어
  (set `SpringArmComponent.CameraLagSpeed` _returnvalue _springarm)
  (set `SpringArmComponent.CameraRotationLagSpeed` _returnvalue _springarm))

(fn `UserConstructionScript`)